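; Networked base shooter character with movement, ADS, health, ragdoll death and a switchable pistol, AR and shotgun loadout.
; Server RPCs handle ammo, reloads and timed fire loops, tracing from camera then muzzle, with cone-spread pellets for shotguns.
; DT_WeaponInfo rows drive weapon stats and visuals, while multicasts play montages and effects and client RPCs refresh HUD ammo.
; Locally controlled Tick sends aim rotation and toggles controller-facing rotation while moving.
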(event Custom|ServerSetADS
  (params (isADS :type Boolean))
  ;[1 0.1297 0.8247] ADS Functionality
  (Variables|Default|SetisADS isADS))

(event Custom|DisableAllInput
  (params (PlayerController :type Player%20Controller%20Object%20Reference))
  ;[0.3294 0 0.6627] Begin play events
  (Input|DisableInput PlayerController))

(event Custom|MC_FireMontage
  ;[0 0 1] Fire weapon events
  (Animation|Montage|PlayMontage (Variables|Character|GetMesh) (Variables|Default|GetChar%20Fire%20Montage)
    (:then
      (Components|Animation|PlayAnimation (Variables|Default|GetWeaponMesh) (Variables|Default|GetWpn%20Fire%20Anim) false))))

(event Custom|PlayReloadMontage
  ;[0.349 1 0.1804] Reload events
  (Networking|SwitchHasAuthority
    (:Authority
      (CallFunction|MCReloadMontage))
    (:Remote
      (CallFunction|ServerReloadMontage))))

(event Custom|Server_ReloadMontage
  ;[0.349 1 0.1804] Reload events
  (CallFunction|MCReloadMontage))

(event Custom|MC_ReloadMontage
  ;[0.349 1 0.1804] Reload events
  (Animation|Montage|PlayMontage (Variables|Character|GetMesh) (Variables|Default|GetChar%20Reload%20Montage)
    (:then
      (Components|Animation|PlayAnimation (Variables|Default|GetWeaponMesh) (Variables|Default|GetWpn%20Reload%20Anim) false))
    (:OnCompleted
      (Variables|Default|SetisReloading false :!label _label))
    (:OnInterrupted
      (goto _label))))

(event Custom|Server_SelectWeapon
  (params (InventoryIndex :type Integer))
  ;[0 1 1] Switch weapon events
  (CallFunction|ServerSetReplicatedWpnVar InventoryIndex)
  (CallFunction|MCSelectWeapon (Utilities|Array|Get(acopy) (Variables|Default|GetWeaponInventoryNames) InventoryIndex)))

(event Custom|MC_SelectWeapon
  (params (WeaponRowName :type Name))
  ;[0 1 1] Switch weapon events
  (CallFunction|SetWeaponDisplayInfo WeaponRowName))

(event Custom|SwitchWeapon
  (params (InventoryIndex :type Integer))
  ;[0 1 1] Switch weapon events
  (Networking|SwitchHasAuthority
    (:Authority
      (CallFunction|MCSwitchWeapon InventoryIndex))
    (:Remote
      (CallFunction|ServerSwitchWeapon InventoryIndex))))

(event Custom|Server_SwitchWeapon
  (params (InventoryIndex :type Integer))
  ;[0 1 1] Switch weapon events
  (CallFunction|MCSwitchWeapon InventoryIndex))

(event Custom|MC_SwitchWeapon
  (params (InventoryIndex :type Integer))
  ;[0 1 1] Switch weapon events
  (if (== (Utilities|Array|Get(acopy) (Variables|Default|GetWeaponInventoryNames) InventoryIndex) "Pistol")
    (Variables|Default|SetCharEquipMontage "/Game/Characters/Heroes/Mannequin/Animations/Actions/MM_Pistol_Equip_Montage.MM_Pistol_Equip_Montage")
    (else
      (Variables|Default|SetCharEquipMontage "/Game/Characters/Heroes/Mannequin/Animations/Actions/MM_Rifle_Equip_Montage.MM_Rifle_Equip_Montage")))
  (Animation|Montage|PlayMontage (Variables|Character|GetMesh) (Variables|Default|GetCharEquipMontage)
    (:then
      (if (Networking|IsServer)
        (Utilities|FlowControl|Delay 0.4)
        (CallFunction|ServerSelectWeapon InventoryIndex)))
    (:OnCompleted
      (Variables|Default|SetisSwitchingWeapons false :!label _label))
    (:OnInterrupted
      (goto _label))))

(event Custom|Server_FireWeaponEvent
  ;[0 0 1] Fire weapon events
  (Utilities|FlowControl|Sequence
    (:then_0
      (CallFunction|MCFireMontage))
    (:then_1
      (CallFunction|MCPlayFireSound))
    (:then_2
      (CallFunction|MCMuzzleFlash))))

(event Custom|Server_FireWeapon
  ;[0 0 1] Fire weapon events
  (bind _canfire (CallFunction|CheckAmmo (Variables|Default|GetActiveWeaponIndex)))
  (if _canfire
    (Variables|Default|SetisFiring true)
    (Variables|Default|SetisFireButtonPressed true)
    (CallFunction|ServerRemoveBulletfromMag (Variables|Default|GetActiveWeaponIndex) :!label _label)
    (CallFunction|ServerBulletTrace)
    (CallFunction|ServerFireWeaponEvent)
    (Utilities|FlowControl|Delay (Variables|Default|GetFire%20Time))
    (bind _canfire_2 (CallFunction|CheckAmmo (Variables|Default|GetActiveWeaponIndex)))
    (if _canfire_2
      (if (and (Variables|Default|GetIs%20Auto%20Fire) (Variables|Default|GetisFireButtonPressed))
        (goto _label)
        (else
          _)))
    (Variables|Default|SetisFiring false)
    (Variables|Default|SetisFireButtonPressed false)))

(event Custom|MC_PlayFireSound
  ;[0 0 1] Fire weapon events
  (Audio|PlaySoundatLocation (Variables|Default|GetFire%20Sound) (Transformation|GetWorldLocation (Variables|Default|GetWeaponMesh)) "0, 0, 0" 0.7 1.0 0.0 0 0 0 0))

(event Custom|MC_MuzzleFlash
  ;[0 0 1] Fire weapon events
  (Effects|SpawnEmitterAttached (Variables|Default|GetMuzzle%20Flash%20FX) (Variables|Default|GetWeaponMesh) (Variables|Default|GetMuzzle%20Socket) "0, 0, 0" "0, 0, 0" "1.000000,1.000000,1.000000" "SnapToTarget"))

(event Custom|Server_ApplyDamage
  (params (DamagedActor :type Actor%20Object%20Reference) (BaseDamage :type Float%20%28single-precision%29) (DamageCauser :type Actor%20Object%20Reference))
  ;[1 0 0] Player damage
  (Game|Damage|ApplyDamage DamagedActor BaseDamage 0 DamageCauser))

(event Custom|MC_BeginPlay
  (params (PlayerController :type Player%20Controller%20Object%20Reference))
  ;[0.3294 0 0.6627] Begin play events
  (bind _asbp_player_controller (Utilities|Casting|CastToBP_PlayerController PlayerController))
  (Variables|Default|SetPlayerController _asbp_player_controller))

(event Custom|Client_RestartLevel
  (CallFunction|ServerRestartLevel))

(event Custom|PlayerDied
  (bind _returnvalue (Utilities|Name|MakeLiteralName "pelvis"))
  (bind _mesh (Variables|Character|GetMesh))
  (bind _charactermovement (Variables|Character|GetCharacterMovement))
  (bind _returnvalue_2 (Pawn|Components|CharacterMovement|GetLastUpdateVelocity _charactermovement))
  ;[1 0 0] Player death event
  (Collision|SetCollisionEnabled (Variables|Collision|GetCapsuleComponent) "NoCollision")
  (Collision|SetCollisionProfileName _mesh "Ragdoll" true :!class /Script/Engine.PrimitiveComponent)
  (Class|SkeletalMeshComponent|SetAllBodiesBelowSimulatePhysics _mesh _returnvalue true true)
  (Physics|AddImpulse _mesh (+ (Math|Vector|Normalize _returnvalue_2) (* _returnvalue_2 "150.000000,150.000000,30.000000")) _returnvalue true)
  (if (Pawn|IsLocallyControlled)
    (bind _asbp_player_controller (Utilities|Casting|CastToBP_PlayerController (Game|GetPlayerController 0)))
    (Input|DisableInput _asbp_player_controller)
    (Actor|Tick|SetActorTickEnabled false)
    (Networking|SwitchHasAuthority
      (:Authority
        (Variables|/Script/Engine.CharacterMovementComponent|SetbUseControllerDesiredRotation (Variables|Character|GetCharacterMovement) false))
      (:Remote
        (CallFunction|ServerSetDesiredRotation false)
        (Variables|/Script/Engine.CharacterMovementComponent|SetbUseControllerDesiredRotation (Variables|Character|GetCharacterMovement) false)))))

(event Custom|Server_RestartLevel
  (bind _asbp_procedural_game_mode (Utilities|Casting|CastToBP_Procedural_GameMode (Game|GetGameMode)))
  (Default|RestartLevel _asbp_procedural_game_mode))

(event Custom|DecrementTeam)

(event Custom|StopFireWeapon
  ;[0 0 1] Fire weapon events
  (Variables|Default|SetisFireButtonPressed false))

(event Custom|Client_UpdateHUD_Clip
  (params (Ammo%20Clip :type Integer))
  ;[0.349 1 0.1804] Reload events
  (Default|UpdateAmmoClip (Variables|Default|GetWBP%20Ingame%20HUD) Ammo%20Clip))

(event Custom|Server_SetDesiredRotation
  (params (Use%20Controller%20Desired%20Rotation :type Boolean))
  ;[1 0.7725 0] Set player rotation
  (Variables|/Script/Engine.CharacterMovementComponent|SetbUseControllerDesiredRotation (Variables|Character|GetCharacterMovement) Use%20Controller%20Desired%20Rotation))

(event Custom|UpdateMoveState
  (params (isMovingThisFrame :type Boolean))
  ;[1 0.7725 0] Set player rotation
  (if (!= isMovingThisFrame (Variables|Default|GetisMoving))
    (Variables|Default|SetisMoving isMovingThisFrame)
    (Networking|SwitchHasAuthority
      (:Authority
        (Variables|/Script/Engine.CharacterMovementComponent|SetbUseControllerDesiredRotation (Variables|Character|GetCharacterMovement) (Variables|Default|GetisMoving)))
      (:Remote
        (CallFunction|ServerSetDesiredRotation (Variables|Default|GetisMoving))
        (Variables|/Script/Engine.CharacterMovementComponent|SetbUseControllerDesiredRotation (Variables|Character|GetCharacterMovement) (Variables|Default|GetisMoving))))
    (else
      (Variables|Default|SetisMoving isMovingThisFrame))))

(event Custom|Server_SetAimRotation
  (params (AimRotation :type Rotator))
  ;[1 0.7725 0] Set player rotation
  (Variables|Default|SetAimRotation AimRotation))

(event Custom|Client_UpdateHUDAmmoStock
  (params (Ammo%20Stock :type Integer))
  ;[0.349 1 0.1804] Reload events
  (Default|UpdateAmmoStock (Variables|Default|GetWBP%20Ingame%20HUD) Ammo%20Stock))

(event Custom|Server_Reload
  ;[0.349 1 0.1804] Reload events
  (CallFunction|ServerReloadAmmo))

(event Game|Damage|EventAnyDamage
  (params (Damage :type Float%20%28single-precision%29) (DamageType :type Damage%20Type%20Object%20Reference) (InstigatedBy :type Controller%20Object%20Reference) (DamageCauser :type Actor%20Object%20Reference))
  ;[1 0 0] Player damage
  (Variables|Default|SetHealth (- (Variables|Default|GetHealth) Damage))
  (if (<= (Variables|Default|GetHealth) 0.0)
    (Utilities|FlowControl|Sequence
      (:then_0
        (CallFunction|PlayerDied)
        (CallFunction|DecrementTeam)))))

(event EventUnpossessed
  (params (OldController :type Controller%20Object%20Reference))
  (Actor|DestroyActor))

(event EventTick
  (params (DeltaSeconds :type Float%20%28single-precision%29))
  ;[0.191 0.5347 1] Event tick
  (CallFunction|UpdateMoveState (> (Math|Vector|VectorLengthXY (Transformation|GetVelocity)) 0.0))
  (Variables|Default|SetNew_AimRotation (Pawn|GetBaseAimRotation))
  (Networking|SwitchHasAuthority
    (:Authority
      (Variables|Default|SetAimRotation (Variables|Default|GetNew_AimRotation)))
    (:Remote
      (CallFunction|ServerSetAimRotation (Variables|Default|GetNew_AimRotation))
      (Variables|Default|SetAimRotation (Variables|Default|GetNew_AimRotation)))))

(event EventPossessed
  (params (NewController :type Controller%20Object%20Reference))
  (bind _asbp_player_controller (Utilities|Casting|CastToBP_PlayerController NewController))
  ;[0.3294 0 0.6627] Begin play events
  (if (Variables|Default|GetDeathRespawn)
    (Variables|Default|SetDeathRespawn false)
    (else
      (CallFunction|DisableAllInput _asbp_player_controller)))
  (CallFunction|MCBeginPlay _asbp_player_controller))

(event EventBeginPlay
  ;[0.3294 0 0.6627] Begin play events
  (Variables|Default|SetStartingPosition (Transformation|GetActorTransform))
  (if (Pawn|IsLocallyControlled)
    _
    (else
      (Actor|Tick|SetActorTickEnabled false)))
  (bind _asabp_character_quinn (Utilities|Casting|CastToABP_Character_Quinn (Components|SkeletalMesh|GetAnimInstance (Variables|Character|GetMesh))))
  (Variables|Default|SetAnimInstance _asabp_character_quinn)
  (if (Networking|IsServer)
    (Utilities|FlowControl|Delay 0.3)
    (CallFunction|ServerAddWpntoInv 0 "Pistol")
    (CallFunction|ServerAddWpntoInv 1 "AR")
    (CallFunction|ServerAddWpntoInv 2 "Shotgun")
    (CallFunction|ServerSelectWeapon)
    (bind _asbp_procedural_game_mode (Utilities|Casting|CastToBP_Procedural_GameMode (Game|GetGameMode)))
    (Variables|/Game/Framework/BP_Procedural_GameMode.BP_Procedural_GameMode_C|SetRespawnTransform _asbp_procedural_game_mode (Transformation|GetActorTransform))))

(event Input|ActionEvents|InputActionADS
  (params (Key :type Key%20Structure :default "None"))
  ;[1 0.1297 0.8247] ADS Functionality
  (:Pressed
    (Networking|SwitchHasAuthority
      (:Authority
        _)
      (:Remote
        (CallFunction|ServerSetADS true)))
    (Variables|Default|SetisADS true))
  (:Released
    (Networking|SwitchHasAuthority
      (:Authority
        _)
      (:Remote
        (CallFunction|ServerSetADS false)))
    (Variables|Default|SetisADS false)))

(event Input|ActionEvents|InputActionFireWeapon
  (params (Key :type Key%20Structure :default "None"))
  ;[0 0 1] Fire weapon events
  (:Pressed
    (if (not (Variables|Default|GetisFiring))
      (CallFunction|ServerFireWeapon)))
  (:Released
    (CallFunction|StopFireWeapon)))

(event Input|ActionEvents|InputActionPauseGame
  (params (Key :type Key%20Structure :default "None"))
  ;[0 1 0.4859] Pause game
  (:Pressed
    (bind _asbp_game_instance (Utilities|Casting|CastToBP_GameInstance (Game|GetGameInstance)))
    (bind _isgamepaused (Default|TogglePauseGame _asbp_game_instance))
    (if _isgamepaused
      (Widget|SetVisibility (Variables|Default|GetWBP%20Ingame%20HUD) "Hidden")
      (else
        (Widget|SetVisibility (Variables|Default|GetWBP%20Ingame%20HUD) "Visible")))))

(event Input|ActionEvents|InputActionReload
  (params (Key :type Key%20Structure :default "None"))
  ;[0.349 1 0.1804] Reload events
  (:Pressed
    (if (not (Variables|Default|GetisReloading))
      (bind _canreload (CallFunction|CheckAmmo (Variables|Default|GetActiveWeaponIndex)))
      (if _canreload
        (Variables|Default|SetisReloading true)
        (CallFunction|PlayReloadMontage)
        (Utilities|FlowControl|Delay (/ (Animation|GetPlayLength (Variables|Default|GetChar%20Reload%20Montage)) 2.0))
        (Networking|SwitchHasAuthority
          (:Authority
            (CallFunction|ServerReloadAmmo))
          (:Remote
            (CallFunction|ServerReload)))))))

(event Input|ActionEvents|InputActionSwitchWeapon
  (params (Key :type Key%20Structure :default "None"))
  ;[0 1 1] Switch weapon events
  (:Pressed
    (if (not (Variables|Default|GetisSwitchingWeapons))
      (Variables|Default|SetisSwitchingWeapons true)
      (if (== (Variables|Default|GetActiveWeaponIndex) (- (Utilities|Array|Length (Variables|Default|GetWeaponInventoryNames)) 1))
        (CallFunction|SwitchWeapon)
        (else
          (CallFunction|SwitchWeapon (+ (Variables|Default|GetActiveWeaponIndex) 1)))))))

(event Input|ActionEvents|InputActionUse
  (params (Key :type Key%20Structure :default "None"))
  (:Pressed
    (Networking|SwitchHasAuthority
      (:Authority
        (CallFunction|ServerRestartLevel))
      (:Remote
        (CallFunction|ClientRestartLevel)))))

(event Input|AxisEvents|InputAxisMoveForward/Backward
  (params (AxisValue :type Float%20%28single-precision%29))
  ;[1 0.4787 0] Movement
  (Pawn|Input|AddMovementInput (Transformation|GetActorForwardVector) AxisValue false))

(event Input|AxisEvents|InputAxisMoveRight/Left
  (params (AxisValue :type Float%20%28single-precision%29))
  ;[1 0.4787 0] Movement
  (Pawn|Input|AddMovementInput (Transformation|GetActorRightVector) AxisValue false))

(event Input|AxisEvents|InputAxisTurnRight/LeftMouse
  (params (AxisValue :type Float%20%28single-precision%29))
  ;[1 0.4787 0] Movement
  (Pawn|Input|AddControllerYawInput AxisValue))

(event Input|AxisEvents|InputAxisLookUp/DownMouse
  (params (AxisValue :type Float%20%28single-precision%29))
  ;[1 0.4787 0] Movement
  (Pawn|Input|AddControllerPitchInput AxisValue))

(fn ConstructionScript)

(fn ServerBulletTrace
  (bind _camera (Variables|Default|GetCamera))
  (bind _weaponmesh (Variables|Default|GetWeaponMesh))
  (bind _muzzle_socket (Variables|Default|GetMuzzle%20Socket))
  (bind _weaponmesh_2 (Variables|Default|GetWeaponMesh))
  (bind _muzzle_socket_2 (Variables|Default|GetMuzzle%20Socket))
  (bind _returnvalue (Transformation|GetWorldTransform _camera))
  (bind _returnvalue_2 (Transformation|GetSocketLocation _weaponmesh _muzzle_socket))
  (bind _returnvalue_3 (Transformation|GetSocketLocation _weaponmesh_2 _muzzle_socket_2))
  (bind (_outhit _returnvalue_4) (Collision|LineTraceByChannel (.location _returnvalue) (+ (.location _returnvalue) (* (Math|Vector|GetForwardVector (.rotation _returnvalue)) 100000)) "TraceTypeQuery2" false 0 "None"))
  (if _returnvalue_4
    (LocalVariables|SetLocal_TargetLocation (.Location (Collision|BreakHitResult _outhit)))
    (else
      (LocalVariables|SetLocal_TargetLocation (.TraceEnd (Collision|BreakHitResult _outhit)))))
  (if (Variables|Default|GetisShotgun)
    (Math|Integer|IncrementInt (LocalVariables|GetLocal_ShotgunShotCount) :!label _label
      (:%20%20
        (bind _outhit_2 (Collision|LineTraceByChannel _returnvalue_3 (+ _returnvalue_3 (* (Math|Random|RandomUnitVectorinConeinDegrees (Math|Vector|GetUnitDirection(Vector) _returnvalue_3 (LocalVariables|GetLocal_TargetLocation)) 3.0) 100000)) "TraceTypeQuery2" false 0 "ForDuration"))
        (Game|Damage|ApplyDamage (.HitActor (Collision|BreakHitResult _outhit_2)) 25.0 0 0)
        (if (< (LocalVariables|GetLocal_ShotgunShotCount) 8)
          (goto _label)
          (else
            (return)))))
    (else
      (bind _outhit_3 (Collision|LineTraceByChannel _returnvalue_2 (+ _returnvalue_2 (* (Math|Vector|GetUnitDirection(Vector) _returnvalue_2 (LocalVariables|GetLocal_TargetLocation)) 100000)) "TraceTypeQuery2" false 0 "ForDuration"))
      (Game|Damage|ApplyDamage (.HitActor (Collision|BreakHitResult _outhit_3)) 25.0 0 0)
      (return))))

(fn ServerAddWpntoInv
  (params (InventorySlot :type Integer) (WeaponRowName :type Name))
  (Utilities|Array|SetArrayElem (Variables|Default|GetWeaponInventoryNames) InventorySlot WeaponRowName true)
  (bind _returnvalue (Utilities|GetDataTableRow "/Game/Weapons/DT_WeaponInfo.DT_WeaponInfo" WeaponRowName)
    (:then
      (Utilities|Array|SetArrayElem (Variables|Default|GetAmmoStockMax) InventorySlot (.AmmoStock (Utilities|Struct|BreakS_WeaponInfo _returnvalue)) true)
      (Utilities|Array|SetArrayElem (Variables|Default|GetAmmoStock) InventorySlot (.AmmoStock (Utilities|Struct|BreakS_WeaponInfo _returnvalue)) true)
      (Utilities|Array|SetArrayElem (Variables|Default|GetAmmoClipMax) InventorySlot (.AmmoClip (Utilities|Struct|BreakS_WeaponInfo _returnvalue)) true)
      (Utilities|Array|SetArrayElem (Variables|Default|GetAmmoClip) InventorySlot (.AmmoClip (Utilities|Struct|BreakS_WeaponInfo _returnvalue)) true)
      (return))))

(fn ServerSetReplicatedWpnVar
  (params (InventoryIndex :type Integer))
  (Variables|Default|SetActiveWeaponIndex InventoryIndex)
  (bind _returnvalue (Utilities|GetDataTableRow "/Game/Weapons/DT_WeaponInfo.DT_WeaponInfo" (Utilities|Array|Get(acopy) (Variables|Default|GetWeaponInventoryNames) InventoryIndex))
    (:then
      (Variables|Default|SetFire%20Time (.FireTime (Utilities|Struct|BreakS_WeaponInfo _returnvalue)))
      (Variables|Default|SetIs%20Auto%20Fire (.isAutoFire (Utilities|Struct|BreakS_WeaponInfo _returnvalue)))
      (Variables|Default|SetIs%20Shotgun (.isShotgun (Utilities|Struct|BreakS_WeaponInfo _returnvalue)))
      (return))))

(fn SetWeaponDisplayInfo
  (params (WeaponRowName :type Name))
  (bind _animinstance (Variables|Default|GetAnimInstance))
  (bind _wbp_ingame_hud (Variables|Default|GetWBP%20Ingame%20HUD))
  (bind _activeweaponindex (Variables|Default|GetActiveWeaponIndex))
  (bind _returnvalue (Utilities|GetDataTableRow "/Game/Weapons/DT_WeaponInfo.DT_WeaponInfo" WeaponRowName)
    (:then
      (Class|SkinnedMeshComponent|SetSkeletalMesh (Variables|Default|GetWeaponMesh) (.WeaponMesh (Utilities|Struct|BreakS_WeaponInfo _returnvalue)) true)
      (Variables|Default|SetFire%20Sound (.FireSound (Utilities|Struct|BreakS_WeaponInfo _returnvalue)))
      (Variables|Default|SetMuzzle%20Socket (.MuzzleSocket (Utilities|Struct|BreakS_WeaponInfo _returnvalue)))
      (Variables|Default|SetShell%20Eject%20Socket (.ShellEjectSocket (Utilities|Struct|BreakS_WeaponInfo _returnvalue)))
      (Variables|Default|SetWpn%20Fire%20Anim (.Wpn_FireAnim (Utilities|Struct|BreakS_WeaponInfo _returnvalue)))
      (Variables|Default|SetWpn%20Reload%20Anim (.Wpn_ReloadAnim (Utilities|Struct|BreakS_WeaponInfo _returnvalue)))
      (Variables|Default|SetChar%20Fire%20Montage (.Char_FireMontage (Utilities|Struct|BreakS_WeaponInfo _returnvalue)))
      (Variables|Default|SetChar%20Reload%20Montage (.Char_ReloadMontage (Utilities|Struct|BreakS_WeaponInfo _returnvalue)))
      (Variables|Default|SetMuzzle%20Flash%20FX (.MuzzleFlash_FX (Utilities|Struct|BreakS_WeaponInfo _returnvalue)))
      (Variables|/Game/Characters/ABP_Character_Quinn.ABP_Character_Quinn_C|SetChar_ADS_Idle _animinstance (.Char_ADS_Idle (Utilities|Struct|BreakS_WeaponInfo _returnvalue)))
      (Variables|/Game/Characters/ABP_Character_Quinn.ABP_Character_Quinn_C|SetChar_Hip_Idle _animinstance (.Char_Hip_Idle (Utilities|Struct|BreakS_WeaponInfo _returnvalue)))
      (Variables|/Game/Characters/ABP_Character_Quinn.ABP_Character_Quinn_C|SetChar_ADS_AO _animinstance (.Char_ADS_AD (Utilities|Struct|BreakS_WeaponInfo _returnvalue)))
      (Variables|/Game/Characters/ABP_Character_Quinn.ABP_Character_Quinn_C|SetChar_Hip_AO _animinstance (.Char_Hip_AO (Utilities|Struct|BreakS_WeaponInfo _returnvalue)))
      (if (Pawn|IsLocallyControlled)
        (Default|UpdateWeaponName _wbp_ingame_hud (Utilities|Text|ToText(Name) (.DisplayName (Utilities|Struct|BreakS_WeaponInfo _returnvalue))))
        (Default|UpdateAmmoClip _wbp_ingame_hud (Utilities|Array|Get(acopy) (Variables|Default|GetAmmoClip) _activeweaponindex))
        (Default|UpdateAmmoStock _wbp_ingame_hud (Utilities|Array|Get(acopy) (Variables|Default|GetAmmoStock) _activeweaponindex))
        (return)))))

(fn ServerRemoveBulletfromMag
  (params (WeaponIndex :type Integer))
  (LocalVariables|SetLocal_NewMagCount (- (Utilities|Array|Get(acopy) (Variables|Default|GetAmmoClip) WeaponIndex) 1))
  (Utilities|Array|SetArrayElem (Variables|Default|GetAmmoClip) WeaponIndex (LocalVariables|GetLocal_NewMagCount))
  (if (Pawn|IsLocallyControlled)
    (Default|UpdateAmmoClip (Variables|Default|GetWBP%20Ingame%20HUD) (LocalVariables|GetLocal_NewMagCount))
    (else
      (CallFunction|ClientUpdateHUDClip (LocalVariables|GetLocal_NewMagCount))))
  (return))

(fn CheckAmmo
  (params (WeaponIndex :type Integer))
  (if (> (Utilities|Array|Get(acopy) (Variables|Default|GetAmmoClip) WeaponIndex) 0)
    (LocalVariables|SetLocal_CanFire true)
    (else
      (LocalVariables|SetLocal_CanFire false)))
  (if (and (> (Utilities|Array|Get(acopy) (Variables|Default|GetAmmoStock) WeaponIndex) 0) (< (Utilities|Array|Get(acopy) (Variables|Default|GetAmmoClip) WeaponIndex) (Utilities|Array|Get(acopy) (Variables|Default|GetAmmoClipMax) WeaponIndex)))
    (LocalVariables|SetLocal_CanReload true)
    (else
      (LocalVariables|SetLocal_CanReload false)))
  (return (LocalVariables|GetLocal_CanFire) (LocalVariables|GetLocal_CanReload)))

(fn ServerReloadAmmo
  (bind _wbp_ingame_hud (Variables|Default|GetWBP%20Ingame%20HUD))
  (LocalVariables|SetLocal_ReloadDifference (- (Utilities|Array|Get(acopy) (Variables|Default|GetAmmoClipMax) (Variables|Default|GetActiveWeaponIndex)) (Utilities|Array|Get(acopy) (Variables|Default|GetAmmoClip) (Variables|Default|GetActiveWeaponIndex))))
  (if (>= (Utilities|Array|Get(acopy) (Variables|Default|GetAmmoStock) (Variables|Default|GetActiveWeaponIndex)) (LocalVariables|GetLocal_ReloadDifference))
    (Utilities|Array|SetArrayElem (Variables|Default|GetAmmoClip) (Variables|Default|GetActiveWeaponIndex) (Utilities|Array|Get(acopy) (Variables|Default|GetAmmoClipMax) (Variables|Default|GetActiveWeaponIndex)))
    (Utilities|Array|SetArrayElem (Variables|Default|GetAmmoStock) (Variables|Default|GetActiveWeaponIndex) (- (Utilities|Array|Get(acopy) (Variables|Default|GetAmmoStock) (Variables|Default|GetActiveWeaponIndex)) (LocalVariables|GetLocal_ReloadDifference)))
    (else
      (Utilities|Array|SetArrayElem (Variables|Default|GetAmmoClip) (Variables|Default|GetActiveWeaponIndex) (+ (Utilities|Array|Get(acopy) (Variables|Default|GetAmmoClip) (Variables|Default|GetActiveWeaponIndex)) (LocalVariables|GetLocal_ReloadDifference)))
      (Utilities|Array|SetArrayElem (Variables|Default|GetAmmoStock) (Variables|Default|GetActiveWeaponIndex) 0)))
  (if (Pawn|IsLocallyControlled)
    (Default|UpdateAmmoClip _wbp_ingame_hud (Utilities|Array|Get(acopy) (Variables|Default|GetAmmoClip) (Variables|Default|GetActiveWeaponIndex)))
    (Default|UpdateAmmoStock _wbp_ingame_hud (Utilities|Array|Get(acopy) (Variables|Default|GetAmmoStock) (Variables|Default|GetActiveWeaponIndex)))
    (return)
    (else
      (CallFunction|ClientUpdateHUDClip (Utilities|Array|Get(acopy) (Variables|Default|GetAmmoClip) (Variables|Default|GetActiveWeaponIndex)))
      (CallFunction|ClientUpdateHUDAmmoStock (Utilities|Array|Get(acopy) (Variables|Default|GetAmmoStock) (Variables|Default|GetActiveWeaponIndex)))
      (return))))