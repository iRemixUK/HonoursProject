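; Game State Blueprint that tracks blue and red team scores and runs the match clock for a team-based game.
; On BeginPlay, the authority starts a one-second looping prematch countdown, which activates the game and starts the match countdown when it expires.
; The match countdown deactivates the game at zero, while a separate event increments either team's score.
; The getters for game status, time, team and scores return placeholder defaults.
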(event Custom|DecrementPrematchTimer
  ;[1 1 1] Prematch Timer
  (bind _result (Math|Integer|DecrementInt (Variables|Default|GetPrematchTime))
    (:%20%20
      (if (<= _result 0)
        (Variables|Default|SetGameIsActive true)
        (Utilities|Time|ClearandInvalidateTimerbyHandle (Variables|Default|GetPrematchTimer))
        ;[1 1 1] Match Timer
        (bind _returnvalue (Utilities|Time|SetTimerbyEvent (delegate Custom|DecrementMatchTimer) 1.0 true))
        (Variables|Default|SetMatchTimer _returnvalue)))))

(event Custom|DecrementMatchTimer
  ;[1 1 1] Match Timer
  (bind _result (Math|Integer|DecrementInt (Variables|Default|GetMatchTime))
    (:%20%20
      (if (<= _result 0)
        (Variables|Default|SetGameIsActive false)
        (Utilities|Time|ClearandInvalidateTimerbyHandle (Variables|Default|GetMatchTimer))))))

(event EventBeginPlay
  ;[1 1 1] Prematch Timer
  (Networking|SwitchHasAuthority
    (:Authority
      (bind _returnvalue (Utilities|Time|SetTimerbyEvent (delegate Custom|DecrementPrematchTimer) 1.0 true))
      (Variables|Default|SetPrematchTimer _returnvalue))))

(event EventIncrementTeamScore
  (params (Team%20Name :type TeamName%20Enum :default "NewEnumerator0"))
  ;[1 1 1] Increment Team Score
  (switch Utilities|FlowControl|Switch|SwitchonTeamName Team%20Name
    (:NewEnumerator0
      (Math|Integer|IncrementInt (Variables|Default|GetTeamBlueScore)))
    (:NewEnumerator1
      (Math|Integer|IncrementInt (Variables|Default|GetTeamRedScore)))))

(fn ConstructionScript)

(fn GetGameIsActive
  (return false))

(fn GetGameTimeRemaining
  (return 0))

(fn GetPlayerScore
  (return 0))

(fn GetTeam
  (return "NewEnumerator0" ""))

(fn GetTeamScore
  (return 0 0))