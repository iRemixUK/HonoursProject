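; Player controller for the menu and multiplayer lobby, handling lobby and character-select UI and the player's profile.
; It loads or creates a saved profile, saves character picks and forwards both to BP_Menu_GameMode through server events.
; Update events refresh player names and level selection in the lobby widget.
; Menus blend the camera between pawn and lobby character; the load screen currently instantiates WBP_LobbyMenu.
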(event Custom|EndClientSession
  (|DestroySession self
    (:then
      (Game|OpenLevel(byName) "MainMenu_Level"))))

(event Custom|CreateLobbyMenu
  (CallFunction|UIDisplayLobbyMenu))

(event Custom|Server_UpdateSelectedCharacter
  (params (PlayerProfileInfo :type S%20Player%20Profile%20Structure))
  (bind _output_get (Variables|Default|SetPlayerProfileInfo PlayerProfileInfo))
  (bind _asbp_menu_game_mode (Utilities|Casting|CastToBP_Menu_GameMode (Game|GetGameMode)))
  (Default|UpdateCharacterforController _asbp_menu_game_mode self _output_get))

(event Custom|InitialSetup
  (CallFunction|LoadSavedProfile)
  (CallFunction|ServerUpdateLobby (Variables|Default|GetPlayerProfileInfo)))

(event Custom|UpdatePlayerNames
  (params (PlayerProfiles :type Array%20of%20S%20Player%20Profile%20Structures))
  (bind _wbp_lobbymenu (Variables|Default|GetWBP_LobbyMenu))
  (Utilities|IsValid _wbp_lobbymenu
    (:Is%20Valid
      (Default|ClearPlayerNames _wbp_lobbymenu)
      (Default|UpdatePlayerNames _wbp_lobbymenu PlayerProfiles))))

(event Custom|Server_SetViewTarget_Normal
  (Game|Player|SetViewTargetwithBlend (Pawn|GetControlledPawn) 0.5 "VTBlend_Linear" 0.0 false))

(event Custom|ServerUpdateLobby
  (params (PlayerProfile :type S%20Player%20Profile%20Structure))
  (Variables|Default|SetPlayerProfileInfo PlayerProfile)
  (bind _asbp_menu_game_mode (Utilities|Casting|CastToBP_Menu_GameMode (Game|GetGameMode)))
  (Default|UpdateLobby _asbp_menu_game_mode true true true))

(event Custom|Server_SetViewTarget_Character
  (Game|Player|SetViewTargetwithBlend (Variables|/Script/Engine.ChildActorComponent|GetChildActor (Variables|/Game/Characters/LobbyCharacter/BP_LobbyCharacter.BP_LobbyCharacter_C|GetViewTarget (Variables|Default|GetLobbyCharacter))) 0.5 "VTBlend_Linear" 0.0 false))

(event Custom|CreateLoadScreen
  (CallFunction|UIDisplayLoadScreen))

(event Custom|UpdateLevelSelection
  (params (LevelRowName :type Name))
  (bind _wbp_lobbymenu (Variables|Default|GetWBP_LobbyMenu))
  (Utilities|IsValid _wbp_lobbymenu
    (:Is%20Valid
      (Default|UpdateLevelSelection _wbp_lobbymenu LevelRowName))))

(event EventBeginPlay
  (if (Pawn|IsLocalController)
    (Variables|Default|SetbShowMouseCursor true)
    (Input|SetInputModeUIOnly self 0 "DoNotLock")))

(event EventTick
  (params (DeltaSeconds :type Float%20%28single-precision%29)))

(fn ConstructionScript)

(fn UIDisplayLobbyMenu
  (Utilities|IsValid (Variables|Default|GetWBP_LobbyMenu)
    (:Is%20Valid
      _)
    (:Is%20Not%20Valid
      (bind _returnvalue (UserInterface|CreateWidget "/Game/Widgets/WBP_LobbyMenu.WBP_LobbyMenu_C" self))
      (Variables|Default|SetWBP_LobbyMenu _returnvalue)))
  (UserInterface|Viewport|AddtoViewport (Variables|Default|GetWBP_LobbyMenu) 0)
  (Networking|SwitchHasAuthority
    (:Authority
      (Game|Player|SetViewTargetwithBlend (Pawn|GetControlledPawn) 0.5 "VTBlend_Linear" 0.0 false))
    (:Remote
      (CallFunction|ServerSetViewTargetNormal)))
  (return))

(fn LoadSavedProfile
  (bind _returnvalue (SaveGame|DoesSaveGameExist (LocalVariables|GetLocal_SlotName)))
  (if _returnvalue
    _
    (else
      (bind _returnvalue_2 (SaveGame|CreateSaveGameObject "/Game/SavedData/SG_PlayerProfile.SG_PlayerProfile_C"))
      (SaveGame|SaveGametoSlot _returnvalue_2 (LocalVariables|GetLocal_SlotName))))
  (bind _returnvalue_3 (SaveGame|LoadGamefromSlot (LocalVariables|GetLocal_SlotName)))
  (bind _assg_player_profile (Utilities|Casting|CastToSG_PlayerProfile _returnvalue_3))
  (Variables|Default|SetPlayerProfileInfo (Variables|/Game/SavedData/SG_PlayerProfile.SG_PlayerProfile_C|GetPlayerProfile _assg_player_profile))
  (return))

(fn UIDisplayLoadScreen
  (Viewport|RemoveAllWidgets)
  (Utilities|IsValid (Variables|Default|GetWBP_LoadScreen)
    (:Is%20Valid
      _)
    (:Is%20Not%20Valid
      (bind _returnvalue (UserInterface|CreateWidget "/Game/Widgets/WBP_LobbyMenu.WBP_LobbyMenu_C" self))
      (Variables|Default|SetWBP_LoadScreen _returnvalue)))
  (UserInterface|Viewport|AddtoViewport (Variables|Default|GetWBP_LoadScreen) 0)
  (return))

(fn UIDisplayCharacterMenu
  (Utilities|IsValid (Variables|Default|GetWBP_CharacterMenu)
    (:Is%20Valid
      _)
    (:Is%20Not%20Valid
      (bind _returnvalue (UserInterface|CreateWidget "/Game/Widgets/WBP_CharacterMenu.WBP_CharacterMenu_C" self))
      (Variables|Default|SetWBP_CharacterMenu _returnvalue)))
  (UserInterface|Viewport|AddtoViewport (Variables|Default|GetWBP_CharacterMenu) 0)
  (Networking|SwitchHasAuthority
    (:Authority
      (Game|Player|SetViewTargetwithBlend (Variables|/Script/Engine.ChildActorComponent|GetChildActor (Variables|/Game/Characters/LobbyCharacter/BP_LobbyCharacter.BP_LobbyCharacter_C|GetViewTarget (Variables|Default|GetLobbyCharacter))) 0.5 "VTBlend_Linear" 0.0 false))
    (:Remote
      (CallFunction|ServerSetViewTargetCharacter)))
  (return))

(fn SaveSelectedCharacter
  (params (RowName :type Name) (CharacterClass :type Actor%20Class%20Reference) (Player%20Profile%20Info%20Team :type E_Team%20Enum :default "NewEnumerator0"))
  (Variables|Default|SetPlayerProfileInfo (Utilities|Struct|MakeS_PlayerProfile (.playername (Variables|Default|GetPlayerProfileInfo)) RowName CharacterClass Player%20Profile%20Info%20Team))
  (Utilities|IsValid (Variables|Default|GetSG_PlayerProfile)
    (:Is%20Valid
      _)
    (:Is%20Not%20Valid
      (bind _returnvalue (SaveGame|CreateSaveGameObject "/Game/SavedData/SG_PlayerProfile.SG_PlayerProfile_C"))
      (Variables|Default|SetSG_PlayerProfile _returnvalue)))
  (Variables|/Game/SavedData/SG_PlayerProfile.SG_PlayerProfile_C|SetPlayerProfile (Variables|Default|GetSG_PlayerProfile) (Variables|Default|GetPlayerProfileInfo))
  (SaveGame|SaveGametoSlot (Variables|Default|GetSG_PlayerProfile) "PlayerProfile_Slot")
  (CallFunction|ServerUpdateSelectedCharacter (Variables|Default|GetPlayerProfileInfo))
  (return))