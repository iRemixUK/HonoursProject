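; Menu game mode that runs the multiplayer lobby, tracking connected menu controllers and their player profiles.
; Players joining the lobby level get a lobby menu, and logouts trigger lobby cleanup.
; UpdateLobby copies profiles into player states and selectively pushes names, level and character changes to all players.
; Character updates spawn each player's lobby character at a free spot, then set its name, mesh and animation from a data table.
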(event Custom|UpdateSelectedCharacter
  (params (PlayerIndex :type Integer))
  (bind _all_connectedplayers (Variables|Default|GetAll_ConnectedPlayers))
  (bind _all_playerprofiles (Variables|Default|GetAll_PlayerProfiles))
  (bind _output (Utilities|Array|Get(acopy) _all_connectedplayers PlayerIndex))
  (bind _output_2 (Utilities|Array|Get(acopy) _all_playerprofiles PlayerIndex))
  (if (== (Variables|/Game/Framework/BP_Menu_Controller.BP_Menu_Controller_C|GetLobbyCharacter (Utilities|Array|Get(acopy) (Variables|Default|GetAll_ConnectedPlayers) PlayerIndex)) 0)
    (bind _available_player_spot (CallFunction|GetLobbyPlayerSpot))
    (Variables|/Game/Characters/LobbyCharacter/BP_PlayerSpotLobby.BP_PlayerSpotLobby_C|SetisSpotUsed _available_player_spot true)
    (bind _returnvalue (Game|SpawnActorfromClass "/Game/Characters/LobbyCharacter/BP_LobbyCharacter.BP_LobbyCharacter_C" (Transformation|GetActorTransform _available_player_spot) "Undefined" 0 0))
    (Variables|/Game/Framework/BP_Menu_Controller.BP_Menu_Controller_C|SetLobbyCharacter _output _returnvalue)
    (Variables|/Game/Framework/BP_Menu_Controller.BP_Menu_Controller_C|SetLobbyPlayerSpot _output _available_player_spot))
  (Default|MCSetPlayerName (Variables|/Game/Framework/BP_Menu_Controller.BP_Menu_Controller_C|GetLobbyCharacter (Utilities|Array|Get(acopy) (Variables|Default|GetAll_ConnectedPlayers) PlayerIndex)) (.playername _output_2))
  (bind _returnvalue_2 (Utilities|GetDataTableRow "/Game/Characters/DT_CharacterInfo.DT_CharacterInfo" (.characterrowname _output_2))
    (:then
      (Default|MCSetCharacterMesh (Variables|/Game/Framework/BP_Menu_Controller.BP_Menu_Controller_C|GetLobbyCharacter (Utilities|Array|Get(acopy) (Variables|Default|GetAll_ConnectedPlayers) PlayerIndex)) (.CharacterMesh (Utilities|Struct|BreakS_CharacterInfo _returnvalue_2)))
      (Default|MCPlayMeshAnim (Variables|/Game/Framework/BP_Menu_Controller.BP_Menu_Controller_C|GetLobbyCharacter (Utilities|Array|Get(acopy) (Variables|Default|GetAll_ConnectedPlayers) PlayerIndex)) (.LobbyAnimation (Utilities|Struct|BreakS_CharacterInfo _returnvalue_2))))))

(event Custom|UpdateLobby
  (params (PlayerNames :type Boolean) (LevelSelection :type Boolean) (CharacterSelection :type Boolean))
  (Utilities|Array|Clear (Variables|Default|GetAll_PlayerProfiles))
  (for (_array_element _array_index) (Variables|Default|GetAll_ConnectedPlayers)
    (Utilities|Array|SetArrayElem (Variables|Default|GetAll_PlayerProfiles) _array_index (Variables|/Game/Framework/BP_Menu_Controller.BP_Menu_Controller_C|GetPlayerProfileInfo _array_element) true)
    (bind _asbp_player_state (Utilities|Casting|CastToBP_PlayerState (Variables|/Script/Engine.Controller|GetPlayerState _array_element)))
    (Variables|/Game/Framework/BP_PlayerState.BP_PlayerState_C|SetPlayerProfile _asbp_player_state (Variables|/Game/Framework/BP_Menu_Controller.BP_Menu_Controller_C|GetPlayerProfileInfo _array_element)))
  (for (_array_element_2 _array_index_2) (Variables|Default|GetAll_ConnectedPlayers)
    (if PlayerNames
      (Default|UpdatePlayerNames _array_element_2 (Variables|Default|GetAll_PlayerProfiles)))
    (if LevelSelection
      (Default|UpdateLevelSelection _array_element_2 (Variables|Default|GetSelectedLevelName)))
    (if CharacterSelection
      (CallFunction|UpdateSelectedCharacter _array_index_2))))

(event Custom|UpdateCharacterForController
  (params (PlayerController :type BP%20Menu%20Controller%20Object%20Reference) (PlayerProfile :type S%20Player%20Profile%20Structure))
  (bind _all_connectedplayers (Variables|Default|GetAll_ConnectedPlayers))
  (bind _returnvalue (Utilities|Array|FindItem _all_connectedplayers PlayerController))
  (Utilities|Array|SetArrayElem (Variables|Default|GetAll_PlayerProfiles) _returnvalue PlayerProfile true)
  (bind _asbp_player_state (Utilities|Casting|CastToBP_PlayerState (Variables|/Script/Engine.Controller|GetPlayerState PlayerController)))
  (Variables|/Game/Framework/BP_PlayerState.BP_PlayerState_C|SetPlayerProfile _asbp_player_state PlayerProfile)
  (CallFunction|UpdateSelectedCharacter _returnvalue))

(event EventBeginPlay)

(event EventTick
  (params (DeltaSeconds :type Float%20%28single-precision%29)))

(event EventHandleStartingNewPlayer
  (params (NewPlayer :type Player%20Controller%20Object%20Reference))
  (bind _returnvalue (Game|GetCurrentLevelName true))
  (switch string _returnvalue
    (:LobbyMenu_Level
      (bind _asbp_menu_controller (Utilities|Casting|CastToBP_Menu_Controller NewPlayer))
      (Utilities|Array|Add (Variables|Default|GetAll_ConnectedPlayers) _asbp_menu_controller)
      (Default|CreateLobbyMenu _asbp_menu_controller)
      (Default|InitialSetup _asbp_menu_controller))))

(event EventOnLogout
  (params (ExitingController :type Controller%20Object%20Reference))
  (bind _asbp_menu_controller (Utilities|Casting|CastToBP_Menu_Controller ExitingController))
  (if (== (Variables|/Game/Framework/BP_Menu_Controller.BP_Menu_Controller_C|GetLobbyCharacter _asbp_menu_controller) 0)
    (Utilities|Array|RemoveItem (Variables|Default|GetAll_ConnectedPlayers) _asbp_menu_controller)
    (CallFunction|UpdateLobby true false true)
    (else
      (Actor|DestroyActor (Variables|/Game/Framework/BP_Menu_Controller.BP_Menu_Controller_C|GetLobbyCharacter _asbp_menu_controller))
      (Variables|/Game/Characters/LobbyCharacter/BP_PlayerSpotLobby.BP_PlayerSpotLobby_C|SetisSpotUsed (Variables|/Game/Framework/BP_Menu_Controller.BP_Menu_Controller_C|GetLobbyPlayerSpot _asbp_menu_controller) false))))

(fn ConstructionScript)

(fn GetLobbyPlayerSpot
  (if (== (Utilities|Array|Length (Variables|Default|GetAll_LobbyPlayerSpots)) 0)
    (bind _outactors (Actor|GetAllActorsOfClass "/Game/Characters/LobbyCharacter/BP_PlayerSpotLobby.BP_PlayerSpotLobby_C"))
    (Variables|Default|SetAll_LobbyPlayerSpots _outactors))
  (bind _array_element (Utilities|Array|ForEachLoopwithBreak (Variables|Default|GetAll_LobbyPlayerSpots) :!label _label)
    (:LoopBody
      (if (not (Variables|/Game/Characters/LobbyCharacter/BP_PlayerSpotLobby.BP_PlayerSpotLobby_C|GetisSpotUsed _array_element))
        (goto _label Break)))
    (:Completed
      (return _array_element))))