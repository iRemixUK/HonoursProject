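; Multiplayer player controller that sets up the local in-game HUD and game-only input, and relays match countdown, start and timer events to that HUD.
; On BeginPlay it loads the saved player profile, setting it directly on authority or sending it to the server from remote clients.
; Respawns go through BP_Procedural_GameMode; possession passes the HUD to the character and replays setup after death.
; It also handles leaving sessions; team getters return placeholder values.
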(event Custom|EnableAllInput
  (Input|EnableInput (Pawn|GetControlledPawn) self))

(event Custom|GameStartCountdown
  (Default|GameStartCountdown (Variables|Default|GetWBP_IngameHUD)))

(event Custom|UnhideIngameHUD
  (Widget|SetVisibility (Variables|Default|GetWBP_IngameHUD) "Visible"))

(event Custom|EndClientSession
  (bind _asbp_game_instance (Utilities|Casting|CastToBP_GameInstance (Game|GetGameInstance)))
  (Variables|/Game/Framework/BP_GameInstance.BP_GameInstance_C|SetMP_IsPauseMenuVisible _asbp_game_instance false)
  (|DestroySession self
    (:then
      (Game|OpenLevel(byName) "MainMenu_Level"))))

(event Custom|Local_SetHUDVariable
  (bind _asbp_character_base (Utilities|Casting|CastToBP_Character_Base (Pawn|GetControlledPawn)))
  (Variables|/Game/Characters/BP_Character_Base.BP_Character_Base_C|SetWBP%20Ingame%20HUD _asbp_character_base (Variables|Default|GetWBP_IngameHUD)))

(event Custom|HUD_StartMatch
  (Default|GMSnDStartMatch (Variables|Default|GetWBP_IngameHUD)))

(event Custom|HUD_SetupMatchTimer
  (params (TimeLeftSec :type Integer))
  (bind _wbp_ingamehud (Variables|Default|GetWBP_IngameHUD))
  (Widget|SetVisibility (Variables|/Game/Widgets/WBP_InGameHUD.WBP_InGameHUD_C|GetText_MatchDuration _wbp_ingamehud) "Visible")
  (Default|UpdateMatchTimer _wbp_ingamehud TimeLeftSec))

(event Custom|RespawnPawn
  (params (Spawn%20Transform :type Transform))
  (Variables|Default|SetDeathRespawn true)
  (bind _asbp_procedural_game_mode (Utilities|Casting|CastToBP_Procedural_GameMode (Game|GetGameMode)))
  (Default|RespawnRequested _asbp_procedural_game_mode self Spawn%20Transform))

(event Custom|MC_BeginPlay
  (if (Pawn|IsLocalPlayerController)
    (Viewport|RemoveAllWidgets)
    (CallFunction|UIShowIngameHud)
    (Input|SetInputModeGameOnly self)
    (Variables|Default|SetbShowMouseCursor false)
    (bind _returnvalue (SaveGame|LoadGamefromSlot "PlayerProfile_Slot"))
    (bind _assg_player_profile (Utilities|Casting|CastToSG_PlayerProfile _returnvalue))
    (Networking|SwitchHasAuthority
      (:Authority
        (Variables|Default|SetPlayer%20Profile (Variables|/Game/SavedData/SG_PlayerProfile.SG_PlayerProfile_C|GetPlayerProfile _assg_player_profile)))
      (:Remote
        (CallFunction|ServerSetPlayerProfile (Variables|/Game/SavedData/SG_PlayerProfile.SG_PlayerProfile_C|GetPlayerProfile _assg_player_profile))))))

(event Custom|Server_SetPlayerProfile
  (params (Player%20Profile :type S%20Player%20Profile%20Structure))
  (Variables|Default|SetPlayer%20Profile Player%20Profile))

(event EventBeginPlay
  (if (Pawn|IsLocalPlayerController)
    (Viewport|RemoveAllWidgets)
    (CallFunction|UIShowIngameHud)
    (Input|SetInputModeGameOnly self)
    (Variables|Default|SetbShowMouseCursor false)
    (bind _returnvalue (SaveGame|LoadGamefromSlot "PlayerProfile_Slot"))
    (bind _assg_player_profile (Utilities|Casting|CastToSG_PlayerProfile _returnvalue))
    (Networking|SwitchHasAuthority
      (:Authority
        (Variables|Default|SetPlayer%20Profile (Variables|/Game/SavedData/SG_PlayerProfile.SG_PlayerProfile_C|GetPlayerProfile _assg_player_profile)))
      (:Remote
        (CallFunction|ServerSetPlayerProfile (Variables|/Game/SavedData/SG_PlayerProfile.SG_PlayerProfile_C|GetPlayerProfile _assg_player_profile))))))

(event EventTick
  (params (DeltaSeconds :type Float%20%28single-precision%29)))

(event EventPossess
  (params (PossessedPawn :type Pawn%20Object%20Reference))
  (CallFunction|LocalSetHUDVariable)
  (if (Variables|Default|GetDeathRespawn)
    (Variables|Default|SetDeathRespawn false)
    (CallFunction|MCBeginPlay)))

(fn ConstructionScript)

(fn UIShowIngameHud
  (Utilities|IsValid (Variables|Default|GetWBP_IngameHUD)
    (:Is%20Valid
      _)
    (:Is%20Not%20Valid
      (bind _returnvalue (UserInterface|CreateWidget "/Game/Widgets/WBP_InGameHUD.WBP_InGameHUD_C" self))
      (Variables|Default|SetWBP_IngameHUD _returnvalue)))
  (UserInterface|Viewport|AddtoViewport (Variables|Default|GetWBP_IngameHUD) 0))

(fn OnRepIsBlue)

(fn GetTeam
  (return "NewEnumerator0" ""))

(fn GetTeamScore
  (return 0 0))