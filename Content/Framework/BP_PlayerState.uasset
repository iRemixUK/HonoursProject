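; Player state that holds a player's profile, team and the round time left for the match HUD.
; CopyProperties carries PlayerProfile over to the new player state, while simple events and getters set and expose the team.
; Timer updates set RoundTimeLeft, whose RepNotify pushes the value to the in-game HUD through the player controller.
; GetAliveTeam and GetTeamScore are stubs that return zero.
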(event Custom|UpdateHUDMatchTimer
  (params (RoundTimeLeft :type Integer))
  (Variables|Default|SetRoundTimeLeft RoundTimeLeft))

(event EventBeginPlay)

(event EventTick
  (params (DeltaSeconds :type Float%20%28single-precision%29)))

(event EventCopyProperties
  (params (NewPlayerState :type Player%20State%20Object%20Reference))
  (bind _asbp_player_state (Utilities|Casting|CastToBP_PlayerState NewPlayerState))
  (Variables|BP_PlayerState_C|SetPlayerProfile _asbp_player_state (Variables|Default|GetPlayerProfile)))

(event EventSetTeam
  (params (Team :type E_Team%20Enum :default "NewEnumerator0"))
  (Variables|Default|SetTeam Team))

(fn ConstructionScript)

(fn OnRepRoundTimeLeft
  (bind _asbp_player_controller (Utilities|Casting|CastToBP_PlayerController (Game|GetPlayerController)))
  (Default|UpdateMatchTimer (Variables|/Game/Framework/BP_PlayerController.BP_PlayerController_C|GetWBP_IngameHUD _asbp_player_controller) (Variables|Default|GetRoundTimeLeft)))

(fn GetAliveTeam
  (params (Team :type E_Team%20Enum :default "NewEnumerator0"))
  (return 0))

(fn GetTeam
  (return (Variables|Default|GetTeam)))

(fn GetTeamScore
  (params (Team :type E_Team%20Enum :default "NewEnumerator0"))
  (return 0))