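; BP_Procedural_GameMode is a game mode that holds the match start until all expected players have arrived, then spawns them.
; It tracks player controllers as they join and leave, taking the expected count from the game instance or one for solo games.
; Each player restarts at a player start named by join index.
; LevelStart then triggers a countdown on every controller and enables input after a short delay.
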(event Custom|LevelStart
  (Utilities|FlowControl|Delay 0.2)
  (for _array_element (Variables|Default|GetAll_ConnectedControllers)
    (Default|GameStartCountdown _array_element))
  (Utilities|FlowControl|Delay 3.0)
  (for _array_element_2 (Variables|Default|GetAll_ConnectedControllers)
    (Default|EnableAllInput _array_element_2)))

(event EventHandleStartingNewPlayer
  (params (NewPlayer :type Player%20Controller%20Object%20Reference))
  (bind _asbp_player_controller (Utilities|Casting|CastToBP_PlayerController NewPlayer))
  (Utilities|Array|Add (Variables|Default|GetAll_ConnectedControllers) _asbp_player_controller)
  (bind _asbp_game_instance (Utilities|Casting|CastToBP_GameInstance (Game|GetGameInstance)))
  (Variables|Default|SetNum_ExpectedPlayers (Variables|/Game/Framework/BP_GameInstance.BP_GameInstance_C|GetNumConnectedPlayers _asbp_game_instance))
  (if (Variables|/Game/Framework/BP_GameInstance.BP_GameInstance_C|GetisSoloGame _asbp_game_instance)
    (Variables|Default|SetNum_ExpectedPlayers 1)
    (Class|GameModeBase|RestartPlayeratPlayerStart (Utilities|Array|Get(acopy) (Variables|Default|GetAll_ConnectedControllers)) (Class|GameModeBase|FindPlayerStart 0 "0"))
    (CallFunction|LevelStart)
    (elif (== (Variables|Default|GetNum_ExpectedPlayers) (Utilities|Array|Length (Variables|Default|GetAll_ConnectedControllers)))
      (Utilities|FlowControl|Delay 0.5)
      (for (_array_element _array_index) (Variables|Default|GetAll_ConnectedControllers)
        (Class|GameModeBase|RestartPlayeratPlayerStart _array_element (Class|GameModeBase|FindPlayerStart _array_element (Utilities|String|ToString(Integer) _array_index))))
      (CallFunction|LevelStart))))

(event EventOnLogout
  (params (ExitingController :type Controller%20Object%20Reference))
  (bind _asbp_player_controller (Utilities|Casting|CastToBP_PlayerController ExitingController))
  (Utilities|Array|RemoveItem (Variables|Default|GetAll_ConnectedControllers) _asbp_player_controller)
  (Math|Integer|DecrementInt (Variables|Default|GetNum_ExpectedPlayers)))

(fn ConstructionScript)