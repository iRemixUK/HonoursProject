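; Game state for a two-team procedural mode, tracking alive counts and scores for Blue defenders and Red attackers.
; On BeginPlay it caches the first player controller and the game mode.
; Events set both alive counts, decrement one team's count and notify the game mode, or increment a team's score.
; Getters return counts and scores per team, while GetTeam always returns Blue.
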(event EventBeginPlay
  (bind _asbp_player_controller (Utilities|Casting|CastToBP_PlayerController (Game|GetPlayerController 0)))
  (Variables|Default|SetAs%20BP%20Player%20Controller _asbp_player_controller)
  (bind _asbp_procedural_game_mode (Utilities|Casting|CastToBP_Procedural_GameMode (Game|GetGameMode)))
  (Variables|Default|SetAs%20BP%20Procedural%20Game%20Mode _asbp_procedural_game_mode))

(event EventTick
  (params (DeltaSeconds :type Float%20%28single-precision%29)))

(event EventIncrementTeamScore
  (params (Team :type E_Team%20Enum :default "NewEnumerator0"))
  (switch Utilities|FlowControl|Switch|SwitchonE_Team Team
    (:NewEnumerator0
      (Math|Integer|IncrementInt (Variables|Default|GetDefenderScore)))
    (:NewEnumerator1
      (Math|Integer|IncrementInt (Variables|Default|GetAttackerScore)))))

(event EventIncrementAliveTeam
  (params (Defenders :type Integer) (Attackers :type Integer))
  (Variables|Default|SetDefendersAlive Defenders)
  (Variables|Default|SetAttackersAlive Attackers))

(event EventDecrementAliveTeam
  (params (Team :type E_Team%20Enum :default "NewEnumerator0"))
  (switch Utilities|FlowControl|Switch|SwitchonE_Team Team
    (:NewEnumerator0
      (Math|Integer|DecrementInt (Variables|Default|GetDefendersAlive)
        (:%20%20
          _)))
    (:NewEnumerator1
      (Math|Integer|DecrementInt (Variables|Default|GetAttackersAlive)
        (:%20%20
          _))))
  (Default|UpdateTeamCount (Variables|Default|GetAs%20BP%20Procedural%20Game%20Mode)))

(fn ConstructionScript)

(fn GetAliveTeam
  (params (Team :type E_Team%20Enum :default "NewEnumerator0"))
  (if (Utilities|Enum|Equal(Enum) Team "NewEnumerator0")
    (return (Variables|Default|GetDefendersAlive))
    (else
      (return (Variables|Default|GetAttackersAlive)))))

(fn GetTeam
  (return "NewEnumerator0"))

(fn GetTeamScore
  (params (Team :type E_Team%20Enum :default "NewEnumerator0"))
  (if (Utilities|Enum|Equal(Enum) Team "NewEnumerator0")
    (return (Variables|Default|GetDefenderScore))
    (else
      (return (Variables|Default|GetAttackerScore)))))