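; Procedural spawner actor that builds a grid map from streamed sublevels on BeginPlay, intended as 10x10 with a wall border.
; A nested loop over LevelGridSize uses hard-coded edge indices to choose between a fixed wall level and a random pick from StreamingLevelNames.
; Each cell creates a uniquely named streaming level instance, positions it by grid index, then loads and shows it.
; The random pick can also return the wall level.
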(event EventBeginPlay
  (bind _levelgridsize (Variables|Default|GetLevelGridSize))
  ;[1 1 1] Loop 100 times to create a 10x10 grid of random levels
  (for _index (range 0 _levelgridsize)
    (for _index_2 (range 0 _levelgridsize)
      (bind _generatewall (CallFunction|ShouldWallbeGenerated? _index _index_2))
      (if _generatewall
        (CallFunction|GenerateWall _index _index_2)
        (else
          (CallFunction|GenerateRandomTile _index _index_2))))))

(event Collision|EventActorBeginOverlap
  (params (OtherActor :type Actor%20Object%20Reference)))

(event EventTick
  (params (DeltaSeconds :type Float%20%28single-precision%29)))

(fn ConstructionScript)

(fn GenerateRandomTile
  (params (IndexX :type Integer) (IndexY :type Integer))
  (bind _streaminglevelnames (Variables|Default|GetStreamingLevelNames))
  ;[1 1 1] Create instance of level, transform it to the correct location, load it and then make it visible
  (bind _returnvalue (Class|LevelStreaming|CreateInstance (Class|GameplayStatics|GetStreamingLevel (Utilities|Array|Get(acopy) _streaminglevelnames (Math|Random|RandomInteger (Utilities|Array|Length _streaminglevelnames)))) (Utilities|String|Append (Utilities|String|ToString(Integer) IndexX) "X" (Utilities|String|ToString(Integer) IndexY))))
  (bind _returnvalue_2 (Class|ProceduralSpawner|MakeTransform IndexX IndexY))
  (Variables|/Script/Engine.LevelStreaming|SetLevelTransform _returnvalue _returnvalue_2)
  (Variables|/Script/Engine.LevelStreaming|SetbShouldBeLoaded _returnvalue true)
  (Variables|/Script/Engine.LevelStreaming|SetbShouldBeVisible _returnvalue true))

(fn GenerateWall
  (params (IndexX :type Integer) (IndexY :type Integer))
  ;[1 1 1] Create instance of level, transform it to the correct location, load it and then make it visible
  (bind _returnvalue (Class|LevelStreaming|CreateInstance (Class|GameplayStatics|GetStreamingLevel (Utilities|Array|Get(acopy) (Variables|Default|GetStreamingLevelNames) 9)) (Utilities|String|Append (Utilities|String|ToString(Integer) IndexX) "X" (Utilities|String|ToString(Integer) IndexY))))
  (bind _returnvalue_2 (Class|ProceduralSpawner|MakeTransform IndexX IndexY))
  (Variables|/Script/Engine.LevelStreaming|SetLevelTransform _returnvalue _returnvalue_2)
  (Variables|/Script/Engine.LevelStreaming|SetbShouldBeLoaded _returnvalue true)
  (Variables|/Script/Engine.LevelStreaming|SetbShouldBeVisible _returnvalue true))

(fn ShouldWallbeGenerated?
  (params (IndexX :type Integer) (IndexY :type Integer))
  ;[1 1 1] Check to see if wall should be generated
  (if (== IndexX 0)
    (return true)
    (elif (== IndexX 9)
      (return true)
      (elif (== IndexY 0)
        (return true)
        (elif (== IndexY 9)
          (return true)
          (else
            (return false)))))))